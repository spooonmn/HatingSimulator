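; Dialogue component for the Damien and Jackie couple in HatingSim, holding their lines as speaker "Couple1".
; Dialouge calls the parent version, then switches on DialougeTreeIndex to pick one of three short exchanges: an entrance remark or one of two opinions on wealth.
; Each exchange shows its reply options through AddDialouge and closes the conversation on Pass Through.
; The two wealth branches then fetch BP_GameManager but do nothing with it.
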(fn `Dialouge`
  (`parent.Dialouge`)
  (switch `int` (`self.DialougeTreeIndex`)
    (:`0`
      (bind (_state _optionsindex) (`self.AddDialouge` "Couple1" "Another couple enters the worst place on earth!" (`|MakeArray` "Good Day M'Lady!" "Have a terrible day!" :!type "Text")))
      (switch `/Game/HatingSim/DialougeImport/DialougeSystem/Enum_DialougeState` _state
        (:`NewEnumerator0`
          (switch `int` _optionsindex
            (:`0`
              (`self.CloseConvo`))
            (:`1`
              (`self.CloseConvo`))))))
    (:`1`
      (bind _state_2 (`self.AddDialouge` "Couple1" "RICH PEOPLE - YUCK" (`|MakeArray` "Imagine hating money..." :!type "Text")))
      (switch `/Game/HatingSim/DialougeImport/DialougeSystem/Enum_DialougeState` _state_2
        (:`NewEnumerator0`
          (`self.CloseConvo`)
          (`GameplayStatics.GetActorOfClass` "/Game/HatingSim/BPs/BP_GameManager.BP_GameManager_C" :!label _label))))
    (:`2`
      (bind _state_3 (`self.AddDialouge` "Couple1" "Anything but expensive things are the best!" (`|MakeArray` "Dang, they like poverty" :!type "Text")))
      (switch `/Game/HatingSim/DialougeImport/DialougeSystem/Enum_DialougeState` _state_3
        (:`NewEnumerator0`
          (`self.CloseConvo`)
          (goto _label))))))