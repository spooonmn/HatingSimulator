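; Dialogue component for the couple Franklin and Margaret, holding their comedic lines and advancing the tutorial.
; After calling the parent Dialouge, it switches on DialougeTreeIndex to pick one of three single-line exchanges with player response options.
; Every response closes the conversation, then finds BP_GameManager, sets its TutorialState and calls ProgressTutorial.
; The first exchange leads to one tutorial state, while the other two share another.
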(fn `Dialouge`
  (`parent.Dialouge`)
  (switch `int` (`self.DialougeTreeIndex`)
    (:`0`
      (bind (_state _optionsindex) (`self.AddDialouge` "Couple1" "Frankkkklin GOONberry is in the house! \n(and margaret)" (`|MakeArray` "What a fantastic name" "I love Gooning!" :!type "Text")))
      (switch `/Game/HatingSim/DialougeImport/DialougeSystem/Enum_DialougeState` _state
        (:`NewEnumerator0`
          (switch `int` _optionsindex
            (:`0`
              (`self.CloseConvo`))
            (:`1`
              (`self.CloseConvo`)))
          (bind _returnvalue (`GameplayStatics.GetActorOfClass` "/Game/HatingSim/BPs/BP_GameManager.BP_GameManager_C"))
          (set `/Game/HatingSim/BPs/BP_GameManager.TutorialState` "NewEnumerator1" _returnvalue)
          (`/Game/HatingSim/BPs/BP_GameManager.ProgressTutorial` _returnvalue))))
    (:`1`
      (bind _state_2 (`self.AddDialouge` "GOONberry and Margaret HATE this microwave" "" (`|MakeArray` "Perfect! Let them FIGHT!" :!type "Text")))
      (switch `/Game/HatingSim/DialougeImport/DialougeSystem/Enum_DialougeState` _state_2
        (:`NewEnumerator0`
          (`self.CloseConvo`)
          (bind _returnvalue_2 (`GameplayStatics.GetActorOfClass` "/Game/HatingSim/BPs/BP_GameManager.BP_GameManager_C" :!label _label))
          (set `/Game/HatingSim/BPs/BP_GameManager.TutorialState` "NewEnumerator4" _returnvalue_2)
          (`/Game/HatingSim/BPs/BP_GameManager.ProgressTutorial` _returnvalue_2))))
    (:`2`
      (bind _state_3 (`self.AddDialouge` "Couple1" "Mr GOONberry gets to GOONing" (`|MakeArray` "That wasn't meant to happen!!" :!type "Text")))
      (switch `/Game/HatingSim/DialougeImport/DialougeSystem/Enum_DialougeState` _state_3
        (:`NewEnumerator0`
          (`self.CloseConvo`)
          (goto _label))))))