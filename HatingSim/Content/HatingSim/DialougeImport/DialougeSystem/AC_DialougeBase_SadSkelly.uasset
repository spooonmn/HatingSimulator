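; Dialogue component for Sad Skelly, an NPC who asks Iso to find a lost bone.
; Its Dialouge override calls the parent, then switches on DialougeTreeIndex between quest request, progress check and random happy lines.
; AddDialouge calls chain through Pass Through states and option indices, then set the tree index or clear progress and close the conversation.
; The bone-return branch, including the switch to the happy stage, is disconnected and never runs.
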(fn `Dialouge`
  (`parent.Dialouge`)
  (switch `int` (`self.DialougeTreeIndex`)
    (:`0`
      (bind _state (`self.AddDialouge` "Sad Skelly" "Im so sad, i cant find my favourite bone"))
      (switch `/Game/HatingSim/DialougeImport/DialougeSystem/Enum_DialougeState` _state
        (:`NewEnumerator0`
          (bind _state_2 (`self.AddDialouge` "Iso" "Dont worry little skelly man, ill find it for you "))
          (switch `/Game/HatingSim/DialougeImport/DialougeSystem/Enum_DialougeState` _state_2
            (:`NewEnumerator0`
              (bind _state_3 (`self.AddDialouge` "Sad Skelly" "THANK YOU ISO Slasher!"))
              (switch `/Game/HatingSim/DialougeImport/DialougeSystem/Enum_DialougeState` _state_3
                (:`NewEnumerator0`
                  (switch `/Game/HatingSim/DialougeImport/DialougeSystem/Enum_DialougeState` "NewEnumerator0"
                    (:`NewEnumerator0`
                      (`self.SetDialougeTreeIndex` 1)
                      (`self.CloseConvo`))))))))))
    (:`1`
      (bind (_state_4 _optionsindex) (`self.AddDialouge` "SadSkelly" "Have you found my bone from the top of the tower \nyet, its really important "))
      (switch `/Game/HatingSim/DialougeImport/DialougeSystem/Enum_DialougeState` _state_4
        (:`NewEnumerator0`
          (switch `int` _optionsindex
            (:`1`
              (bind _state_5 (`self.AddDialouge` "SadSkelly" "Well i Hope you find it soon im so sad:<"))
              (switch `/Game/HatingSim/DialougeImport/DialougeSystem/Enum_DialougeState` _state_5
                (:`NewEnumerator0`
                  (`self.SetDialougeTreeIndex` 1)
                  (`self.CloseConvo`))))))))
    (:`2`
      (bind _state_6 (`self.AddDialouge` "Happy Skelly" (`KismetArrayLibrary.Array_Random` (`|MakeArray` "I love My Bone " "Ill never let my bone out of my sight again" "I love my boner.. i mean bone " :!type "Text"))))
      (switch `/Game/HatingSim/DialougeImport/DialougeSystem/Enum_DialougeState` _state_6
        (:`NewEnumerator0`
          (`self.ClearDialougeProgress`)
          (`self.CloseConvo`))))))