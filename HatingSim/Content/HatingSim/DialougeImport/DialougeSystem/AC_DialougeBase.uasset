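; Base dialogue component that runs branching conversations through a UW_Dialouge widget and pauses player control while one is open.
; The empty Dialouge function is a hook for scripts, which replay from the start each time an option is selected.
; AddDialouge returns saved choices from the DialougeProgress map for answered steps, otherwise sends the line and options to the widget.
; Helpers clear or rewind progress, and changing the tree index resets it.
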(fn `AddDialouge`
  (params (Speaker :type Text) (Dialouge :type Text) (OptionsText :type "Array of Text"))
  (returns (State :type "/Game/HatingSim/DialougeImport/DialougeSystem/Enum_DialougeState Enum") (OptionsIndex :type Integer))
  (bind (_value _returnvalue) (`BlueprintMapLibrary.Map_Find` (`self.DialougeProgress`) (`self.DialougeIndex`)))
  (`/Engine/EditorBlueprintResources/StandardMacros.IncrementInt` (`self.DialougeIndex`)
    (:`  `
      (if _returnvalue
        (return "NewEnumerator0" _value)
        (else
          (`/Game/HatingSim/DialougeImport/UI/Dialouge/UW_Dialouge.UpdateDialougeText` (`self.DialougeWidget`) (`self.DialougeIndex`) (`self.CoupleSpeaker`) (`local.Dialouge`) (`local.OptionsText`))
          (return "NewEnumerator1" 0))))))

(fn `ClearDialougeProgress`
  (`BlueprintMapLibrary.Map_Clear` (`self.DialougeProgress`)))

(fn `CloseConvo`
  (bind _returnvalue (`GameplayStatics.GetPlayerController` 0))
  (`Widget.RemoveFromParent` (`self.DialougeWidget`))
  (set `PlayerController.bShowMouseCursor` false _returnvalue)
  (`WidgetBlueprintLibrary.SetInputMode_GameOnly` _returnvalue)
  (`self.UnpausePlayer`)
  (`self.OnDialougeClose`))

(fn `Dialouge`)

(fn `OpenConvo`
  (bind _returnvalue (`|CreateWidget` "/Game/HatingSim/DialougeImport/UI/Dialouge/UW_Dialouge.UW_Dialouge_C" (`GameplayStatics.GetPlayerController` 0) self))
  (bind _output_get (set `self.DialougeWidget` _returnvalue))
  (`UserWidget.AddToViewport` _output_get 0)
  (`self.ProgressDialouge`)
  (`self.PausePlayer`))

(fn `PausePlayer`
  (bind _returnvalue (`GameplayStatics.GetPlayerCharacter` 0))
  (`Controller.SetIgnoreMoveInput` (`GameplayStatics.GetPlayerController` 0) true)
  (`Actor.DisableInput` _returnvalue (`GameplayStatics.GetPlayerController` 0))
  (`MovementComponent.StopMovementImmediately` (`Character.CharacterMovement` _returnvalue))
  (`WidgetBlueprintLibrary.SetInputMode_UIOnlyEx` (`GameplayStatics.GetPlayerController` 0) (`self.DialougeWidget`))
  (set `PlayerController.bShowMouseCursor` true (`GameplayStatics.GetPlayerController` 0)))

(fn `ProgressDialouge`
  (set `self.DialougeIndex` -1)
  (`self.Dialouge`))

(fn `RemoveDialougeProgress`
  (params (ProgressSteps :type Integer))
  (for _index (range (+ ProgressSteps 1))
    (`BlueprintMapLibrary.Map_Remove` (`self.DialougeProgress`) (- (`self.DialougeIndex`) _index))))

(fn `SetDialougeTreeIndex`
  (params (DialougeTreeIndex :type Integer))
  (set `self.DialougeTreeIndex` DialougeTreeIndex)
  (`self.ClearDialougeProgress`))

(fn `UnpausePlayer`
  (set `PlayerController.bShowMouseCursor` false (`GameplayStatics.GetPlayerController` 0))
  (`WidgetBlueprintLibrary.SetInputMode_GameOnly` (`GameplayStatics.GetPlayerController` 0))
  (`Controller.SetIgnoreMoveInput` (`GameplayStatics.GetPlayerController` 0) false)
  (`Actor.EnableInput` (`GameplayStatics.GetPlayerCharacter` 0) (`GameplayStatics.GetPlayerController` 0)))

(fn `UpdateSelectedOption`
  (params (ProgressIndex :type "Integer (by ref)") (OptionIndex :type "Integer (by ref)"))
  (`BlueprintMapLibrary.Map_Add` (`self.DialougeProgress`) ProgressIndex OptionIndex)
  (`self.ProgressDialouge`))