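; Tutorial dialogue component for the restaurant couple the player is tasked with ruining the date of.
; It overrides the parent Dialouge function and picks one of three hard-coded exchanges by DialougeTreeIndex.
; Any reply closes the conversation, then sets TutorialState on BP_GameManager and calls ProgressTutorial.
; Both greeting replies advance to the same state, and the two later exchanges share another.
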(fn `Dialouge`
  (`parent.Dialouge`)
  (switch `int` (`self.DialougeTreeIndex`)
    (:`0`
      (bind (_state _optionsindex) (`self.AddDialouge` "Couple1" "Michael and Pete arrive \nat the restaurant. Your job  \nis to ruin their date. How  \ndo you greet them?" (`|MakeArray` "Bonjour and welcome!" "I love your hair!" :!type "Text")))
      (switch `/Game/HatingSim/DialougeImport/DialougeSystem/Enum_DialougeState` _state
        (:`NewEnumerator0`
          (switch `int` _optionsindex
            (:`0`
              (`self.CloseConvo`))
            (:`1`
              (`self.CloseConvo`)))
          (bind _returnvalue (`GameplayStatics.GetActorOfClass` "/Game/HatingSim/BPs/BP_GameManager.BP_GameManager_C"))
          (set `/Game/HatingSim/BPs/BP_GameManager.TutorialState` "NewEnumerator1" _returnvalue)
          (`/Game/HatingSim/BPs/BP_GameManager.ProgressTutorial` _returnvalue))))
    (:`1`
      (bind _state_2 (`self.AddDialouge` "Couple1" "YOU HATE UNITY! BUT LOVE UNREAL! \nI HATE YOU!" (`|MakeArray` "HAHA I love CHAOS" :!type "Text")))
      (switch `/Game/HatingSim/DialougeImport/DialougeSystem/Enum_DialougeState` _state_2
        (:`NewEnumerator0`
          (`self.CloseConvo`)
          (bind _returnvalue_2 (`GameplayStatics.GetActorOfClass` "/Game/HatingSim/BPs/BP_GameManager.BP_GameManager_C" :!label _label))
          (set `/Game/HatingSim/BPs/BP_GameManager.TutorialState` "NewEnumerator4" _returnvalue_2)
          (`/Game/HatingSim/BPs/BP_GameManager.ProgressTutorial` _returnvalue_2))))
    (:`2`
      (bind _state_3 (`self.AddDialouge` "Couple1" "They start knoodling aggresively" (`|MakeArray` "Oh YEAH!" :!type "Text")))
      (switch `/Game/HatingSim/DialougeImport/DialougeSystem/Enum_DialougeState` _state_3
        (:`NewEnumerator0`
          (`self.CloseConvo`)
          (goto _label))))))