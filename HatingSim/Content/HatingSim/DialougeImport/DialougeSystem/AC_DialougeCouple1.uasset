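; Dialogue component for the Couple1 speaker in HatingSim, holding that character's conversations.
; The Dialouge function calls its parent, then switches on DialougeTreeIndex to pick a greeting as a new couple, an angry Unity-versus-Unreal outburst or a pleased remark.
; Each branch passes its line and player reply options to AddDialouge, and on Pass Through every reply closes the conversation.
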(fn `Dialouge`
  (`parent.Dialouge`)
  (switch `int` (`self.DialougeTreeIndex`)
    (:`0`
      (bind (_state _optionsindex) (`self.AddDialouge` "Couple1" "Hello! Nice to meet you were a new couple" (`|MakeArray` "Bonjour!" "Yeah, we'll see about that..." :!type "Text")))
      (switch `/Game/HatingSim/DialougeImport/DialougeSystem/Enum_DialougeState` _state
        (:`NewEnumerator0`
          (switch `int` _optionsindex
            (:`0`
              (`self.CloseConvo`))
            (:`1`
              (`self.CloseConvo`))))))
    (:`1`
      (bind _state_2 (`self.AddDialouge` "Couple1" "YOU HATE UNITY! BUT LOVE UNREAL! \nI HATE YOU!" (`|MakeArray` "Mwahaha" :!type "Text")))
      (switch `/Game/HatingSim/DialougeImport/DialougeSystem/Enum_DialougeState` _state_2
        (:`NewEnumerator0`
          (`self.CloseConvo`))))
    (:`2`
      (bind _state_3 (`self.AddDialouge` "Couple1" "hehe, i love these things! " (`|MakeArray` "Mwahaha" :!type "Text")))
      (switch `/Game/HatingSim/DialougeImport/DialougeSystem/Enum_DialougeState` _state_3
        (:`NewEnumerator0`
          (`self.CloseConvo`))))))