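; Dialogue component for the Brian and Tim couple in HatingSim, holding their short date-related conversations.
; Overrides Dialouge, calls the parent, then switches on DialougeTreeIndex to show one of three lines from Couple1 with player reply options: an opener, a hated-meat reaction or a happy reaction.
; Every reply closes the conversation; the two reaction branches then look up BP_GameManager but do nothing further with it.
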(fn `Dialouge`
  (`parent.Dialouge`)
  (switch `int` (`self.DialougeTreeIndex`)
    (:`0`
      (bind (_state _optionsindex) (`self.AddDialouge` "Couple1" "briannnnnnnnnnnnnn" (`|MakeArray` "Oui!" "I hope you don't enjoy your date!" :!type "Text")))
      (switch `/Game/HatingSim/DialougeImport/DialougeSystem/Enum_DialougeState` _state
        (:`NewEnumerator0`
          (switch `int` _optionsindex
            (:`0`
              (`self.CloseConvo`))
            (:`1`
              (`self.CloseConvo`))))))
    (:`1`
      (bind _state_2 (`self.AddDialouge` "Couple1" "AHH i HATE MEAT" (`|MakeArray` "YES, I hope you had a terrible date!" :!type "Text")))
      (switch `/Game/HatingSim/DialougeImport/DialougeSystem/Enum_DialougeState` _state_2
        (:`NewEnumerator0`
          (`self.CloseConvo`)
          (`GameplayStatics.GetActorOfClass` "/Game/HatingSim/BPs/BP_GameManager.BP_GameManager_C" :!label _label))))
    (:`2`
      (bind _state_3 (`self.AddDialouge` "Couple1" "this is the best. i love you!" (`|MakeArray` "NOO you were meant to hate that!" :!type "Text")))
      (switch `/Game/HatingSim/DialougeImport/DialougeSystem/Enum_DialougeState` _state_3
        (:`NewEnumerator0`
          (`self.CloseConvo`)
          (goto _label))))))