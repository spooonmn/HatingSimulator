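; Game manager for Hating Simulator that runs the date-ruining tutorial and spawns couples into the scene.
; ProgressTutorial updates the tutorial widget by TutorialState, toggles guest list and item cues, then activates the game.
; Tick switches on GameState, spawning a fixed tutorial couple, then random couples through a DoOnce re-armed by random delays and coin flips.
; SpawnCouple assigns each couple a random free table from those gathered at BeginPlay.
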(event `ProgressTutorial`
  (switch `/Game/HatingSim/BPs/E_TutorialStates` (`self.TutorialState`) :!label _label
    (:`NewEnumerator0`
      (set `TextBlock.Text` "● Welcome to Hating Simulator!   \n \nA couple has just walked in! Why dont you try talking to them?" (`/Game/HatingSim/UW_Tutorial.TextBlock` (`self.TutorialWidget`))))
    (:`NewEnumerator1`
      (set `TextBlock.Text` "● Tutorial 2/5 \n \nWhat a lovley couple, lets check the Guest List to see what things  \nthey like and dislike" (`/Game/HatingSim/UW_Tutorial.TextBlock` (`self.TutorialWidget`)))
      (`/Game/HatingSim/BPs/BP_GuestListObject.ToggleTut` (`self.GuestList`) true))
    (:`NewEnumerator2`
      (set `TextBlock.Text` "● Tutorial 3/5 \n \nIt seems like one of them loves Unreal Engine, but the other one loves Unity, how about we ruin their date and give them a game console so they fight about it! \n \nPick up the Console in the back and give it to them." (`/Game/HatingSim/UW_Tutorial.TextBlock` (`self.TutorialWidget`)))
      (`/Game/HatingSim/BPs/Items/BP_GameConsole.ToggleTut` (`self.Object`) true))
    (:`NewEnumerator3`
      (set `TextBlock.Text` "● Tutorial 4/5 \n \nYou found the Game Console! Now just give it to them and see what happens!" (`/Game/HatingSim/UW_Tutorial.TextBlock` (`self.TutorialWidget`))))
    (:`NewEnumerator4`
      (set `TextBlock.Text` "● Tutorial 5/5 \n \nNow you can try it on your own, ruin as many couples dates and relationships as possible before they have a good time and leave!" (`/Game/HatingSim/UW_Tutorial.TextBlock` (`self.TutorialWidget`)))
      (`KismetSystemLibrary.Delay` 10.0)
      (`Widget.RemoveFromParent` (`self.TutorialWidget`))
      (`self.SetGameState` "NewEnumerator2"))))

(event `self.ReceiveBeginPlay`
  (`self.GetAllTablesInScene`)
  (bind _returnvalue (`|CreateWidget` "/Game/HatingSim/UW_Tutorial.UW_Tutorial_C"))
  (bind _output_get (set `self.TutorialWidget` _returnvalue))
  (`UserWidget.AddToViewport` _output_get 0)
  (goto _label))

(event `self.ReceiveTick`
  (params (DeltaSeconds :type "Float (single-precision)"))
  (switch `/Game/HatingSim/BPs/E_GameStates` (`self.GameState`)
    (:`NewEnumerator1`
      (`KismetSystemLibrary.Delay` 0.0)
      (`self.SetGameState` "NewEnumerator4"))
    (:`NewEnumerator4`
      (`/Engine/EditorBlueprintResources/StandardMacros.DoOnce` false
        (:`Completed`
          (`self.SpawnCouple` "/Game/HatingSim/BPs/Couple/BP_CoupleBrianTim.BP_CoupleBrianTim_C"))))
    (:`NewEnumerator2`
      (`/Engine/EditorBlueprintResources/StandardMacros.DoOnce` false :!label _label_2
        (:`Completed`
          (`self.SpawnCouple` (`KismetArrayLibrary.Array_Random` (`self.AllCouples`)))
          (`KismetSystemLibrary.Delay` (`KismetMathLibrary.RandomFloatInRange` 2.0 4.5) :!label _label_3)
          (if (<= (`KismetMathLibrary.RandomFloatInRange` 0.0 1.0) 0.5)
            (goto _label_2 :!via `Reset`)
            (else
              (goto _label_3))))))))

(event `SpawnCouple`
  (params (CoupleToSpawn :type "/Game/HatingSim/BPs/Couple/BP_Couple Class Reference") (Remove :type Boolean))
  (bind (_randomunassignedtable _success) (`self.GetRandomUnassignedTable`))
  (if _success
    (bind _returnvalue (`|SpawnActorFromClass` CoupleToSpawn (`self.GetTransform`) "Undefined" "MultiplyWithRoot" null (`/Game/HatingSim/BPs/BP_TableBase.TableID` _randomunassignedtable) null))
    (set `/Game/HatingSim/BPs/BP_TableBase.IsAssigned?` true _randomunassignedtable)
    (`KismetArrayLibrary.Array_Add` (`self.ActiveCouples`) _returnvalue)
    (if Remove
      (`KismetArrayLibrary.Array_RemoveItem` (`self.AllCouples`) CoupleToSpawn))))

(fn `GetAllTablesInScene`
  ;[1 1 1] Remove talbes from list then find all in scene and add to list
  (`KismetArrayLibrary.Array_Clear` (`self.TableList`))
  (bind _outactors (`GameplayStatics.GetAllActorsOfClass` "/Game/HatingSim/BPs/BP_TableBase.BP_TableBase_C"))
  (`KismetArrayLibrary.Array_Append` (`self.TableList`) _outactors))

(fn `GetRandomUnassignedTable`
  (returns (RandomUnassignedTable :type "/Game/HatingSim/BPs/BP_TableBase Object Reference") (Success :type Boolean))
  (locals (UnassignedTables :type "Array of /Game/HatingSim/BPs/BP_TableBase Object Reference"))
  (`KismetArrayLibrary.Array_Clear` (`local.UnassignedTables`))
  (for _array_element (`self.TableList`)
    (if (not (`/Game/HatingSim/BPs/BP_TableBase.IsAssigned?` _array_element))
      (`KismetArrayLibrary.Array_Add` (`local.UnassignedTables`) _array_element)))
  (if (`KismetArrayLibrary.Array_IsNotEmpty` (`local.UnassignedTables`))
    (return (`KismetArrayLibrary.Array_Random` (`local.UnassignedTables`)) true)
    (else
      (return null false))))

(fn `SetGameState`
  (params (GameState :type "/Game/HatingSim/BPs/E_GameStates Enum" :default "NewEnumerator0"))
  (set `self.GameState` GameState))

(fn `UserConstructionScript`)