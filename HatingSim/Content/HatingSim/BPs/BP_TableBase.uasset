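; Restaurant-style table actor that seats an assigned NPC couple and handles the player's interactions with them.
; Overlapping NPCs with a matching table ID take both seats, then interacting opens dialogue, adds a guest-list slide and starts a timer-driven heart bar.
; A handed-over item picks the correct or wrong dialogue branch, with particles hiding the couple.
; The couple walks home after that dialogue or when the bar completes, freeing the table.
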(event `self.ReceiveTick`
  (params (DeltaSeconds :type "Float (single-precision)")))

(event `Rot`
  (bind _text (`self.Text`))
  (bind (_returnvalue_location _returnvalue_rotation) (`KismetMathLibrary.BreakTransform` (`SceneComponent.K2_GetComponentToWorld` (`/Game/HatingSim/BPs/BP_PlayerCharacter.FollowCamera` (`self.Player`)))))
  (`SceneComponent.K2_SetWorldRotation` _text _returnvalue_rotation false false)
  (`SceneComponent.K2_AddLocalRotation` :`self` _text))

(event `self.ReceiveBeginPlay`
  (bind _heartbar (`self.HeartBar`))
  (bind _returnvalue (`SceneComponent.K2_GetComponentToWorld` (`/Game/HatingSim/BPs/BP_PlayerCharacter.FollowCamera` (`self.Player`))))
  (bind _asbp_player_character (cast `/Game/HatingSim/BPs/BP_PlayerCharacter` (`GameplayStatics.GetPlayerCharacter` 0)))
  (set `self.Player` _asbp_player_character)
  (`self.Rot`)
  (bind _returnvalue_2 (`|SpawnActorFromClass` "/Game/HatingSim/BPs/BP_NavMeshPoint.BP_NavMeshPoint_C" (`SceneComponent.K2_GetComponentToWorld` (`self.NavMeshTarget`)) "Undefined" "MultiplyWithRoot" null null))
  (set `self.NavMeshPointActor` _returnvalue_2)
  (`SceneComponent.K2_SetWorldRotation` _heartbar (`KismetMathLibrary.MakeRotator` (* (.roll (.rotation _returnvalue)) -1.0) (.pitch (.rotation _returnvalue)) (.yaw (.rotation _returnvalue))) false false)
  (`SceneComponent.K2_AddLocalRotation` :`self` _heartbar))

(event `self.CoupleSitTrigger.OnComponentBeginOverlap`
  (params (OverlappedComponent :type "PrimitiveComponent Object Reference") (OtherActor :type "Actor Object Reference") (OtherComp :type "PrimitiveComponent Object Reference") (OtherBodyIndex :type Integer) (bFromSweep :type Boolean) (SweepResult :type "HitResult Structure (by ref)"))
  (bind _asbp_npc (cast `/Game/HatingSim/BPs/Couple/BP_NPC` OtherActor))
  (set `self.CoupleAtTable` (`/Game/HatingSim/BPs/Couple/BP_NPC.Couple` _asbp_npc))
  (if (== (`self.TableID`) (`/Game/HatingSim/BPs/Couple/BP_NPC.TargetTableID` _asbp_npc))
    (if (== (`self.TempCouple1`) _asbp_npc)
      _
      (elif (`self.Seat1Full`)
        (if (not (`self.Seat2Full`))
          (`/Game/HatingSim/BPs/Couple/BP_NPC.SitOnSeat` _asbp_npc (`SceneComponent.K2_GetComponentToWorld` (`self.SeatLeft`)))
          (set `self.Seat2Full` true)
          (set `self.IsOcupied` true)
          (`/Game/HatingSim/BPs/Couple/BP_Couple.SetCoupleState` (`self.CoupleAtTable`) "NewEnumerator2")
          (`SceneComponent.SetVisibility` (`self.Text`) true false)
          (bind _output_get (set `self.TempCouple2` _asbp_npc))
          (`MovementComponent.StopMovementImmediately` (`Character.CharacterMovement` _output_get))
          (`/Game/HatingSim/BPs/Couple/BP_NPC.ToggleLegRot` (`self.TempCouple2`) true)
          (`GameplayStatics.SpawnSound2D` "/Game/HatingSim/SFX/Sounds/sitting_on_chair_Cue.sitting_on_chair_Cue" 1.0 1.0 0.0 null))
        (else
          (`/Game/HatingSim/BPs/Couple/BP_NPC.SitOnSeat` _asbp_npc (`SceneComponent.K2_GetComponentToWorld` (`self.SeatRight`)))
          (set `self.Seat1Full` true)
          (bind _output_get_2 (set `self.TempCouple1` _asbp_npc))
          (`MovementComponent.StopMovementImmediately` (`Character.CharacterMovement` _output_get_2))
          (`/Game/HatingSim/BPs/Couple/BP_NPC.ToggleLegRot` (`self.TempCouple1`) true)
          (`GameplayStatics.PlaySound2D` "/Game/HatingSim/SFX/Sounds/sitting_on_chair_Cue.sitting_on_chair_Cue" 1.0 1.0 0.0 null null))))))

(event `self.CoupleSitTrigger.OnComponentHit`
  (params (HitComponent :type "PrimitiveComponent Object Reference") (OtherActor :type "Actor Object Reference") (OtherComp :type "PrimitiveComponent Object Reference") (NormalImpulse :type "Vector Structure") (Hit :type "HitResult Structure (by ref)")))

(event `/Game/HatingSim/BPs/INterface/BPI_Interactable.Interact`
  (params (Instigator :type "Actor Object Reference"))
  (bind _coupleattable (`self.CoupleAtTable`))
  (bind _coupleattable_2 (`self.CoupleAtTable`)
    (:`then`
      (switch `/Game/HatingSim/BPs/Couple/E_CoupleStates` (`/Game/HatingSim/BPs/Couple/BP_Couple.CoupleStates` _coupleattable_2)
        (:`NewEnumerator2`
          (add `/Game/HatingSim/DialougeImport/DialougeSystem/AC_DialougeBase.OnDialougeClose` (`/Game/HatingSim/BPs/Couple/BP_Couple.DialougeComponent` (`self.CoupleAtTable`)) (delegate `FadeOutDialouge`))
          (`/Game/HatingSim/DialougeImport/DialougeSystem/AC_DialougeBase.OpenConvo` (`/Game/HatingSim/BPs/Couple/BP_Couple.DialougeComponent` (`self.CoupleAtTable`)))
          (bind _returnvalue (`GameplayStatics.SpawnSound2D` "/Game/HatingSim/SFX/Sounds/OpenDialougeCue.OpenDialougeCue" 1.0 1.0 0.0 null))
          (set `self.CurrentlyPlayingSound` _returnvalue)
          (`/Game/HatingSim/BPs/Couple/BP_Couple.SetCoupleState` (`self.CoupleAtTable`) "NewEnumerator3")
          (`SceneComponent.SetVisibility` (`self.Text`) false false)
          (bind _returnvalue_2 (`GameplayStatics.GetActorOfClass` "/Game/HatingSim/BPs/BP_GuestListObject.BP_GuestListObject_C"))
          (`/Game/HatingSim/BPs/BP_GuestListObject.AddCoupleInfoSlide` _returnvalue_2 (`/Game/HatingSim/BPs/Couple/BP_Couple.CouplePic` _coupleattable) (`/Game/HatingSim/BPs/Couple/BP_Couple.CoupleName` _coupleattable) (`/Game/HatingSim/BPs/Couple/BP_Couple.LikesText` _coupleattable) (`/Game/HatingSim/BPs/Couple/BP_Couple.LikesText1` _coupleattable) (`/Game/HatingSim/BPs/Couple/BP_Couple.DislikesText` _coupleattable) (`/Game/HatingSim/BPs/Couple/BP_Couple.DislikesText1` _coupleattable) (`self.TableID`))
          (`SceneComponent.SetVisibility` (`self.HeartBar`) true false)
          (bind _asuw_heart_progress_bar (cast `/Game/HatingSim/UW_HeartProgressBar` (`WidgetComponent.GetWidget` (`self.HeartBar`))))
          (set `self.healthbar` _asuw_heart_progress_bar)
          (bind _returnvalue_3 (`KismetSystemLibrary.K2_SetTimerDelegate` (delegate `UpdateProgressBar`) 0.1 true true))
          (set `self.ProgressBarTimer` _returnvalue_3))
        (:`NewEnumerator3`
          (`self.FadeOutDialouge`)
          (if (`/Game/HatingSim/BPs/BP_PlayerCharacter.HandsFull` (`self.Player`))
            (`self.GiveHeldItem` (`/Game/HatingSim/BPs/BP_PlayerCharacter.HeldItem` (`self.Player`)))
            (`KismetSystemLibrary.K2_ClearAndInvalidateTimerHandle` (`self.ProgressBarTimer`))))
        (:`NewEnumerator4`
          (`/Game/HatingSim/BPs/Couple/BP_Couple.SetCoupleState` _coupleattable_2 "NewEnumerator2"))))
    (:`else`)))

(event `UpdateProgressBar`
  (bind _finished_ (`/Game/HatingSim/UW_HeartProgressBar.UpdateBar1` (`self.healthbar`)))
  (if _finished_
    (`KismetSystemLibrary.K2_ClearAndInvalidateTimerHandle` (`self.ProgressBarTimer`))
    (`/Game/HatingSim/BPs/Couple/BP_Couple.SetCoupleState` (`self.CoupleAtTable`) "NewEnumerator5")
    (`self.WalkCoupleHome`)
    (`SceneComponent.SetVisibility` (`self.HeartBar`) false false)))

(event `FadeOutDialouge`
  (bind _currentlyplayingsound (`self.CurrentlyPlayingSound`)
    (:`then`
      (`AudioComponent.FadeOut` _currentlyplayingsound 0.5 0.0 "Linear")
      (remove `/Game/HatingSim/DialougeImport/DialougeSystem/AC_DialougeBase.OnDialougeClose` (`/Game/HatingSim/BPs/Couple/BP_Couple.DialougeComponent` (`self.CoupleAtTable`)) (delegate `FadeOutDialouge`)))
    (:`else`)))

(event `GiveHeldItem`
  (params (Item :type "/Game/HatingSim/BPs/Items/BP_ItemBase Object Reference"))
  (bind _dialougecomponent (`/Game/HatingSim/BPs/Couple/BP_Couple.DialougeComponent` (`self.CoupleAtTable`)))
  (if (== (`GameplayStatics.GetObjectClass` Item) (`/Game/HatingSim/BPs/Couple/BP_Couple.CorrectItem` (`self.CoupleAtTable`)))
    (bind _returnvalue (`AddComponent|NODE_AddNiagaraComponent-2` :`RelativeTransform` (`SceneComponent.GetRelativeTransform` (`self.ParticleEffectPOS`))))
    (set `self.NiagaraParticle` _returnvalue)
    (bind _returnvalue_2 (`GameplayStatics.SpawnSound2D` "/Game/HatingSim/SFX/Sounds/couple_fight_Cue.couple_fight_Cue" 1.0 1.0 0.0 null))
    (set `self.CurrentlyPlayingSound` _returnvalue_2)
    (`/Game/HatingSim/DialougeImport/DialougeSystem/AC_DialougeBase.SetDialougeTreeIndex` _dialougecomponent 1)
    (else
      (bind _returnvalue_3 (`AddComponent|NODE_AddNiagaraComponent-1` :`RelativeTransform` (`SceneComponent.GetRelativeTransform` (`self.ParticleEffectPOS`))))
      (set `self.NiagaraParticle` _returnvalue_3)
      (`/Game/HatingSim/DialougeImport/DialougeSystem/AC_DialougeBase.SetDialougeTreeIndex` _dialougecomponent 2)))
  (`/Game/HatingSim/DialougeImport/DialougeSystem/AC_DialougeBase.OpenConvo` (`/Game/HatingSim/BPs/Couple/BP_Couple.DialougeComponent` (`self.CoupleAtTable`)))
  (`self.ToggleMeshVis` false)
  (`/Game/HatingSim/BPs/BP_PlayerCharacter.DestroyItem` (`self.Player`))
  (`/Game/HatingSim/BPs/Couple/BP_Couple.SetCoupleState` (`self.CoupleAtTable`) "NewEnumerator4")
  (`SceneComponent.SetVisibility` (`self.HeartBar`) false false)
  (`ProgressBar.SetPercent` (`/Game/HatingSim/UW_HeartProgressBar.ProgressBar_0` (`self.healthbar`)) 0.0)
  (add `/Game/HatingSim/DialougeImport/DialougeSystem/AC_DialougeBase.OnDialougeClose` (`/Game/HatingSim/BPs/Couple/BP_Couple.DialougeComponent` (`self.CoupleAtTable`)) (delegate `OnDialougeClose_Event`))
  (bind _returnvalue_4 (`GameplayStatics.GetActorOfClass` "/Game/HatingSim/BPs/BP_GuestListObject.BP_GuestListObject_C"))
  (`/Game/HatingSim/BPs/BP_GuestListObject.DestorySlideAtID` _returnvalue_4 (`self.TableID`)))

(event `WalkCoupleHome`
  (bind _coupleattable (`self.CoupleAtTable`))
  (set `self.TempCouple1` (`/Game/HatingSim/BPs/Couple/BP_Couple.Person1` _coupleattable))
  (set `self.TempCouple2` (`/Game/HatingSim/BPs/Couple/BP_Couple.Person2` _coupleattable))
  (`/Game/HatingSim/BPs/Couple/BP_NPC.WalkHome` (`self.TempCouple1`) (`SceneComponent.K2_GetComponentLocation` (`self.P1Leave`)))
  (`/Game/HatingSim/BPs/Couple/BP_NPC.WalkHome` (`self.TempCouple2`) (`SceneComponent.K2_GetComponentLocation` (`self.P2Leave`)))
  (`KismetSystemLibrary.Delay` 3.0)
  (set `self.IsAssigned?` false)
  (set `self.Seat1Full` false)
  (set `self.Seat2Full` false)
  (set `self.IsOcupied` false)
  (set `self.CoupleAtTable` null))

(event `OnDialougeClose_Event`
  (remove `/Game/HatingSim/DialougeImport/DialougeSystem/AC_DialougeBase.OnDialougeClose` (`/Game/HatingSim/BPs/Couple/BP_Couple.DialougeComponent` (`self.CoupleAtTable`)) (delegate `OnDialougeClose_Event`))
  (`KismetSystemLibrary.Delay` 3.0)
  (`self.ToggleMeshVis` true)
  (bind _currentlyplayingsound (`self.CurrentlyPlayingSound`)
    (:`then`
      (`AudioComponent.FadeOut` _currentlyplayingsound 0.5 0.0 "Linear"))
    (:`else`
      _))
  (`|ExecutionSequence`
    (:`then_0`
      (`self.WalkCoupleHome`)
      (`/Game/HatingSim/BPs/Couple/BP_NPC.ToggleLegRot` (`self.TempCouple1`) false)
      (`/Game/HatingSim/BPs/Couple/BP_NPC.ToggleLegRot` (`self.TempCouple2`) false))
    (:`then_1`
      (`NiagaraComponent.SetPaused` (`self.NiagaraParticle`) true)
      (`ActorComponent.K2_DestroyComponent` (`self.NiagaraParticle`)))))

(event `ToggleMeshVis`
  (params (Toggle :type Boolean))
  (bind _coupleattable (`self.CoupleAtTable`))
  (`SceneComponent.SetVisibility` (`/Game/HatingSim/BPs/Couple/BP_NPC.NpcMesh` (`/Game/HatingSim/BPs/Couple/BP_Couple.Person1` _coupleattable)) Toggle true)
  (`SceneComponent.SetVisibility` (`/Game/HatingSim/BPs/Couple/BP_NPC.NpcMesh` (`/Game/HatingSim/BPs/Couple/BP_Couple.Person2` _coupleattable)) Toggle true))

(fn `UserConstructionScript`)