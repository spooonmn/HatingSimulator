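; BP_NPC is an NPC that walks to a table location using AI movement.
; Tick waits until TableLocation is non-zero, then a DoOnce gate issues a single AIMoveTo on itself toward that point.
; Debug prints report the destination, the start of the move and its success or failure.
; The file does not set TableLocation itself.
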(event `self.ReceiveTick`
  (params (DeltaSeconds :type "Float (single-precision)"))
  (if (!= (`self.TableLocation`) (0.0 0.0 0.0))
    (`/Engine/EditorBlueprintResources/StandardMacros.DoOnce` false
      (:`Completed`
        (`|AIMoveTo` self (`self.TableLocation`) null 25.0
          (:`then`
            (`KismetSystemLibrary.PrintString` (`KismetStringLibrary.Conv_VectorToString` (`self.TableLocation`)))
            (`KismetSystemLibrary.PrintString` "started"))
          (:`OnSuccess`
            (`KismetSystemLibrary.PrintString` "suc"))
          (:`OnFail`
            (`KismetSystemLibrary.PrintString` "fail")))))))

(fn `UserConstructionScript`)