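; BP_Couple is a spawner actor that creates a pair of NPCs bound for the same table.
; On BeginPlay it spawns two BP_NPC at Spawn1 and Spawn2, passing each the target table ID, itself and a table location.
; FindTableLocation scans all BP_TableBase actors for the matching TableID and returns its nav point's world location.
; Both spawns are stored in Person1, so only the second reference is kept.
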(event `self.ReceiveBeginPlay`
  (`self.SpawnNPCs`))

(event `SpawnNPCs`
  (bind _transform (`self.FindTableLocation`))
  (bind _returnvalue (`|SpawnActorFromClass` "/Game/HatingSim/BPs/BP_NPC.BP_NPC_C" (`SceneComponent.K2_GetComponentToWorld` (`self.Spawn1`)) "Undefined" "MultiplyWithRoot" null (`self.TargetTableID`) self _transform null))
  (set `self.Person1` _returnvalue)
  (bind _transform_2 (`self.FindTableLocation`))
  (bind _returnvalue_2 (`|SpawnActorFromClass` "/Game/HatingSim/BPs/BP_NPC.BP_NPC_C" (`SceneComponent.K2_GetComponentToWorld` (`self.Spawn2`)) "Undefined" "MultiplyWithRoot" null (`self.TargetTableID`) self _transform_2 null))
  (set `self.Person1` _returnvalue_2))

(fn `FindTableLocation`
  (returns (Transform :type "Vector Structure"))
  (bind _outactors (`GameplayStatics.GetAllActorsOfClass` "/Game/HatingSim/BPs/BP_TableBase.BP_TableBase_C"))
  (for _array_element _outactors
    (if (== (`/Game/HatingSim/BPs/BP_TableBase.TableID` _array_element) (`self.TargetTableID`))
      (return (`SceneComponent.K2_GetComponentLocation` (`/Game/HatingSim/BPs/BP_NavMeshPoint.DefaultSceneRoot` (`/Game/HatingSim/BPs/BP_TableBase.NavMeshPointActor` _array_element)))))))

(fn `UserConstructionScript`)