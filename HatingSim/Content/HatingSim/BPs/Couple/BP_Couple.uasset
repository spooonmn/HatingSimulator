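; BP_Couple is an actor representing a couple in HatingSim, made up of two NPCs and a shared dialogue component.
; On BeginPlay it sets an initial couple state, then spawns two BP_NPC actors at its Spawn1 and Spawn2 transforms.
; Each NPC receives the TargetTableID and a reference back to the couple.
; A DialougeTree component is then added at runtime with its speaker set to CoupleName.
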(event `self.ReceiveBeginPlay`
  (`self.SpawnNPCs`)
  (bind _returnvalue (`|AddComponentByClass` (`self.DialougeTree`)))
  (bind _output_get (set `self.DialougeComponent` _returnvalue))
  (set `/Game/HatingSim/DialougeImport/DialougeSystem/AC_DialougeBase.CoupleSpeaker` (`self.CoupleName`) _output_get))

(event `SpawnNPCs`
  (`self.SetCoupleState` "NewEnumerator1")
  (bind _returnvalue (`|SpawnActorFromClass` "/Game/HatingSim/BPs/Couple/BP_NPC.BP_NPC_C" (`SceneComponent.K2_GetComponentToWorld` (`self.Spawn1`)) "Undefined" "MultiplyWithRoot" null (`self.TargetTableID`) self (0.0 0.0 0.0) null))
  (set `self.Person1` _returnvalue)
  (bind _returnvalue_2 (`|SpawnActorFromClass` "/Game/HatingSim/BPs/Couple/BP_NPC.BP_NPC_C" (`SceneComponent.K2_GetComponentToWorld` (`self.Spawn2`)) "Undefined" "MultiplyWithRoot" null (`self.TargetTableID`) self (0.0 0.0 0.0) null))
  (set `self.Person2` _returnvalue_2))

(fn `SetCoupleState`
  (params (CoupleState :type "/Game/HatingSim/BPs/Couple/E_CoupleStates Enum" :default "NewEnumerator0"))
  (set `self.CoupleStates` CoupleState))

(fn `UserConstructionScript`)