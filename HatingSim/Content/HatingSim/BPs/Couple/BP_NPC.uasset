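; BP_NPC is a character, part of a couple, that walks to its assigned table and later walks home.
; Tick resolves the table's nav point by TargetTableID, then issues one AI move there.
; WalkHome moves it beside the table, walks it to the game manager, then destroys it, removing its couple from ActiveCouples if either partner is invalid.
; Random walk speed, delayed head bob and sound, and sit/stand leg mesh swapping handle presentation.
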(event `ToggleLegRot`
  (params (Sit :type Boolean))
  (`SceneComponent.SetVisibility` (`self.EvilMC_Legs_001`) (not Sit) false)
  (`SceneComponent.SetVisibility` (`self.EvilMC_Legs_sit`) Sit false))

(event `HeadBob`
  (`KismetSystemLibrary.Delay` (`KismetMathLibrary.RandomFloatInRange` 0.1 0.3))
  (bind (_direction _newtrack_0) (`Timeline|bob`)
    (:`Update`
      (`SceneComponent.K2_SetRelativeLocation` (`self.Upper`) (`KismetMathLibrary.MakeVector` 0.0 0.0 (+ (* _newtrack_0 2.0) -10.0)) false false))))

(event `self.ReceiveBeginPlay`
  (`|ExecutionSequence`
    (:`then_0`
      (`self.HeadBob`)
      (set `CharacterMovementComponent.MaxWalkSpeed` (`KismetMathLibrary.RandomFloatInRange` 150.0 250.0) (`self.CharacterMovement`))
      (bind _returnvalue (`GameplayStatics.GetActorOfClass` "/Game/HatingSim/BPs/BP_GameManager.BP_GameManager_C"))
      (set `self.GameManager` _returnvalue)
      (bind _asbp_player_character (cast `/Game/HatingSim/BPs/BP_PlayerCharacter` (`GameplayStatics.GetPlayerCharacter` 0)))
      (set `self.As BP Player Character` _asbp_player_character))
    (:`then_1`
      (`KismetSystemLibrary.Delay` (`KismetMathLibrary.RandomFloatInRange` 0.1 0.3))
      (`GameplayStatics.PlaySoundAtLocation` "/Game/HatingSim/SFX/Sounds/SpawnCue.SpawnCue" (`self.K2_GetActorLocation`) (struct) 1.0 1.0 0.0 null null null null))))

(event `self.ReceiveTick`
  (params (DeltaSeconds :type "Float (single-precision)"))
  (if (!= (`self.TableLocation`) (0.0 0.0 0.0))
    (`/Engine/EditorBlueprintResources/StandardMacros.DoOnce` false
      (:`Completed`
        (`|AIMoveTo` self (`self.TableLocation`) null 25.0)))
    (else
      (bind _transform (`self.FindTableLocation`))
      (set `self.TableLocation` _transform))))

(event `WalkHome`
  (params (SideOfTableLoc :type "Vector Structure"))
  (bind _couple (`self.Couple`))
  (if (!= (`self.TableLocation`) (0.0 0.0 0.0))
    (`self.K2_SetActorLocation` SideOfTableLoc)
    (`|AIMoveTo` self (`self.K2_GetActorLocation` (`self.GameManager`)) null 40.0
      (:`OnSuccess`
        (if (or (not (`KismetSystemLibrary.IsValid` (`/Game/HatingSim/BPs/Couple/BP_Couple.Person1` _couple))) (not (`KismetSystemLibrary.IsValid` (`/Game/HatingSim/BPs/Couple/BP_Couple.Person2` _couple))))
          (bind _returnvalue (`GameplayStatics.GetActorOfClass` "/Game/HatingSim/BPs/BP_GameManager.BP_GameManager_C"))
          (`KismetArrayLibrary.Array_RemoveItem` (`/Game/HatingSim/BPs/BP_GameManager.ActiveCouples` _returnvalue) (`self.Couple`)))
        (`self.K2_DestroyActor`)))
    (else
      (`KismetSystemLibrary.Delay` 3.0)
      (`self.K2_DestroyActor`))))

(fn `FindTableLocation`
  (returns (Transform :type "Vector Structure"))
  (bind _outactors (`GameplayStatics.GetAllActorsOfClass` "/Game/HatingSim/BPs/BP_TableBase.BP_TableBase_C"))
  (for _array_element _outactors
    (if (== (`/Game/HatingSim/BPs/BP_TableBase.TableID` _array_element) (`self.TargetTableID`))
      (return (`SceneComponent.K2_GetComponentLocation` (`/Game/HatingSim/BPs/BP_NavMeshPoint.DefaultSceneRoot` (`/Game/HatingSim/BPs/BP_TableBase.NavMeshPointActor` _array_element)))))))

(fn `SitOnSeat`
  (params (Transform :type "Transform Structure"))
  (`SceneComponent.K2_SetWorldTransform` (`self.CapsuleComponent`) Transform false true))

(fn `UserConstructionScript`)