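; BP_GuestListObject is an interactable guest list that opens a tablet UI showing couples' pictures, names, likes and dislikes.
; It creates a hidden UW_Tablet at BeginPlay, forwards couple slides to it, and turns its prompt text toward the camera once.
; Interact plays the intro animation and enables the cursor; the first use also advances BP_GameManager's tutorial.
; Leaving the sphere restores game input and plays the exit animation before hiding the tablet.
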(event `Rot`
  (bind _text (`self.Text`))
  (bind _asbp_player_character (cast `/Game/HatingSim/BPs/BP_PlayerCharacter` (`GameplayStatics.GetPlayerCharacter` 0)))
  (bind (_returnvalue_location _returnvalue_rotation) (`KismetMathLibrary.BreakTransform` (`SceneComponent.K2_GetComponentToWorld` (`/Game/HatingSim/BPs/BP_PlayerCharacter.FollowCamera` _asbp_player_character))))
  (`SceneComponent.K2_SetWorldRotation` _text _returnvalue_rotation false false)
  (`SceneComponent.K2_AddLocalRotation` :`self` _text))

(event `ToggleMouseInput`
  (params (Toggle :type Boolean))
  (bind _output_get (set `PlayerController.bShowMouseCursor` Toggle (`GameplayStatics.GetPlayerController` 0)))
  (if _output_get
    (`WidgetBlueprintLibrary.SetInputMode_GameAndUIEx` (`GameplayStatics.GetPlayerController` 0) null "DoNotLock" true true)
    (else
      (`WidgetBlueprintLibrary.SetInputMode_GameOnly` (`GameplayStatics.GetPlayerController` 0)))))

(event `self.ReceiveBeginPlay`
  (bind _returnvalue (`|CreateWidget` "/Game/HatingSim/UW_Tablet.UW_Tablet_C"))
  (bind _output_get (set `self.Tablet` _returnvalue))
  (`Widget.SetVisibility` _output_get "Hidden")
  (`UserWidget.AddToViewport` _output_get 0)
  (`self.Rot`))

(event `/Game/HatingSim/BPs/INterface/BPI_Interactable.Interact`
  (params (Instigator :type "Actor Object Reference"))
  (`self.ResetLeaveSound`)
  (`GameplayStatics.PlaySound2D` "/Game/HatingSim/SFX/Sounds/ui_hover_Cue.ui_hover_Cue" 1.0 1.0 0.0 null null)
  (`self.Tablet`
    (:`then`
      (if (not (`self.UIActive`))
        (`Widget.SetVisibility` (`self.Tablet`) "Visible")
        (`/Game/HatingSim/UW_Tablet.PlayIntroAnim` (stale _output_get) :!label _label)
        (`self.ToggleMouseInput` true)
        (set `self.UIActive` true)
        (`/Engine/EditorBlueprintResources/StandardMacros.DoOnce` false
          (:`Completed`
            (bind _returnvalue (`GameplayStatics.GetActorOfClass` "/Game/HatingSim/BPs/BP_GameManager.BP_GameManager_C"))
            (set `/Game/HatingSim/BPs/BP_GameManager.TutorialState` "NewEnumerator2" _returnvalue)
            (`self.ToggleTut` false)
            (`/Game/HatingSim/BPs/BP_GameManager.ProgressTutorial` _returnvalue)))))
    (:`else`
      (bind _returnvalue_2 (`|CreateWidget` "/Game/HatingSim/UW_Tablet.UW_Tablet_C"))
      (`UserWidget.AddToViewport` _returnvalue_2 0)
      (bind _output_get (set `self.Tablet` _returnvalue_2))
      (goto _label))))

(event `ToggleTut`
  (params (Show :type Boolean))
  (`SceneComponent.SetVisibility` (`self.Text`) Show false))

(event `self.Sphere.OnComponentEndOverlap`
  (params (OverlappedComponent :type "PrimitiveComponent Object Reference") (OtherActor :type "Actor Object Reference") (OtherComp :type "PrimitiveComponent Object Reference") (OtherBodyIndex :type Integer))
  (if (== OtherActor (`GameplayStatics.GetPlayerCharacter` 0))
    (`self.RemoveUI`)))

(event `RemoveUI`
  (bind _tablet (`self.Tablet`))
  (`self.Tablet`
    (:`then`
      (`self.ToggleMouseInput` false)
      (set `self.UIActive` false)
      (`/Engine/EditorBlueprintResources/StandardMacros.DoOnce` true :!label _label_2
        (:`Completed`
          (`GameplayStatics.PlaySound2D` "/Game/HatingSim/SFX/Sounds/ui_click_Cue.ui_click_Cue" 1.0 1.0 0.0 null null)
          (`/Game/HatingSim/UW_Tablet.ReverseAnim` _tablet)
          (add `/Game/HatingSim/UW_Tablet.FinishedOutAnim` _tablet (delegate `FinishedOutAnim_Event`)))))
    (:`else`)))

(event `AddCoupleInfoSlide`
  (params (CouplePic :type "Texture2D Object Reference") (CoupleName :type Text) (Likes1 :type Text) (Likes2 :type Text) (Dislikes1 :type Text) (Dislikes2 :type Text))
  (`/Game/HatingSim/UW_Tablet.AddCoupleInfoSlide` (`self.Tablet`) CouplePic CoupleName Likes1 Likes2 Dislikes1 Dislikes2))

(event `ResetLeaveSound`
  (goto _label_2 :!via `Reset`))

(event `FinishedOutAnim_Event`
  (bind _tablet (`self.Tablet`))
  (`Widget.SetVisibility` _tablet "Hidden")
  (remove `/Game/HatingSim/UW_Tablet.FinishedOutAnim` _tablet (delegate `FinishedOutAnim_Event`)))

(fn `UserConstructionScript`)