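; BP_ItemBase is an item Actor that the player picks up by interacting with it.
; Interact checks that the item is not held and the BP_PlayerCharacter's hands are not full, then, through a DoOnce, stores the instigator, calls BePickedUp and plays a pickup sound.
; BePickedUp hands the item to that character's PickUp function.
; An unreached SpawnActor node that would duplicate the item remains in the graph.
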(event `BePickedUp`
  (bind _asbp_player_character (cast `/Game/HatingSim/BPs/BP_PlayerCharacter` (`self.Player`)))
  (`/Game/HatingSim/BPs/BP_PlayerCharacter.PickUp` _asbp_player_character self))

(event `/Game/HatingSim/BPs/INterface/BPI_Interactable.Interact`
  (params (Instigator :type "Actor Object Reference"))
  (bind _asbp_player_character (cast `/Game/HatingSim/BPs/BP_PlayerCharacter` Instigator))
  (if (and (not (`self.BeingHeld`)) (not (`/Game/HatingSim/BPs/BP_PlayerCharacter.HandsFull` _asbp_player_character)))
    (`/Engine/EditorBlueprintResources/StandardMacros.DoOnce` false
      (:`Completed`
        (set `self.Player` Instigator)
        (`self.BePickedUp`)
        (`GameplayStatics.PlaySound2D` "/Game/HatingSim/SFX/Sounds/item_pickup_Cue.item_pickup_Cue" 1.0 1.0 0.0 null null)))))

(fn `UserConstructionScript`)