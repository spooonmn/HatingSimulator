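; BP_GameConsole is an interactable game console pickup that advances the game's tutorial.
; When interacted with while not already held, it stores the player, gets picked up, sets the game manager's tutorial state, progresses it and plays a pickup sound.
; A separate event toggles the visibility of its text render, used as a tutorial prompt.
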(event `ToggleTut`
  (params (Show :type Boolean))
  (`SceneComponent.SetVisibility` (`self.TextRender`) Show false))

(event `/Game/HatingSim/BPs/INterface/BPI_Interactable.Interact`
  (params (Instigator :type "Actor Object Reference"))
  (if (not (`self.BeingHeld`))
    (set `self.Player` Instigator)
    (`self.BePickedUp`)
    (bind _returnvalue (`GameplayStatics.GetActorOfClass` "/Game/HatingSim/BPs/BP_GameManager.BP_GameManager_C"))
    (set `/Game/HatingSim/BPs/BP_GameManager.TutorialState` "NewEnumerator3" _returnvalue)
    (`/Game/HatingSim/BPs/BP_GameManager.ProgressTutorial` _returnvalue)
    (`GameplayStatics.PlaySound2D` "/Game/HatingSim/SFX/Sounds/item_pickup_Cue.item_pickup_Cue" 1.0 1.0 0.0 null null)))

(fn `UserConstructionScript`
  (`parent.UserConstructionScript`))